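; Game mode for a two-player VR match that drives the countdown, finish, reset and leave flow through multicast RPCs on NewGameStateBase.
; It starts the countdown once two button presses are counted, and resetting players clears that count.
; On finish, it computes a position in front of each VR pawn, facing back at it, to pass with the winner.
; ChoosePlayerStart assigns spawns sequentially by matching indexed PlayerStart tags.
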(event `Increment Counter`
  (bind _result (`/Engine/EditorBlueprintResources/StandardMacros.IncrementInt` (`self.NumButtonPressed`))
    (:`  `
      (bind _output_get (set `self.NumButtonPressed` _result))
      (if (>= _output_get 2)
        (bind _asnew_game_state_base (cast `/Game/Assignment3/Blueprints/NewGameStateBase` (`GameplayStatics.GetGameState`))
          (:`then`
            (`/Game/Assignment3/Blueprints/NewGameStateBase.RPC_Multicast_StartCountdown` _asnew_game_state_base))
          (:`CastFailed`
            (`KismetSystemLibrary.PrintString` "Game State Base Cast Failed")))))))

(event `Display Finish Message`
  (params (Client0Won :type Boolean))
  (bind _arrayrotator (`self.ArrayRotator`))
  (bind _arraylocation (`self.ArrayLocation`))
  (bind _outactors (`GameplayStatics.GetAllActorsOfClass` "/Script/Engine.PlayerController"))
  (for (_array_element _array_index) _outactors
    (bind _asbp_vrpawn (cast `/Game/Assignment3/Blueprints/BP_VRPawn` (`Controller.K2_GetPawn` _array_element))
      (:`then`
        (bind _returnvalue (`self.GetActorForwardVector` _asbp_vrpawn))
        (`KismetArrayLibrary.Array_Set` (`self.ArrayRotator`) _array_index (`KismetMathLibrary.MakeRotFromX` (* _returnvalue (-1.0 -1.0 -1.0))) true)
        (`KismetArrayLibrary.Array_Set` (`self.ArrayLocation`) _array_index (+ (`SceneComponent.K2_GetComponentLocation` (`/Game/Assignment3/Blueprints/BP_VRPawn.Camera` _asbp_vrpawn)) (* _returnvalue (150.0 150.0 150.0))) true))
      (:`CastFailed`
        (`KismetSystemLibrary.PrintString` "cast failed"))))
  (bind _asnew_game_state_base (cast `/Game/Assignment3/Blueprints/NewGameStateBase` (`GameplayStatics.GetGameState`))
    (:`then`
      (`/Game/Assignment3/Blueprints/NewGameStateBase.RPC_Multicast_FinishMessage` _asnew_game_state_base Client0Won (`|GetArrayItem` _arrayrotator) (`|GetArrayItem` _arrayrotator 1) (`|GetArrayItem` _arraylocation) (`|GetArrayItem` _arraylocation 1)))
    (:`CastFailed`
      (`KismetSystemLibrary.PrintString` "Cast failed"))))

(event `ResetPlayers`
  (bind _asnew_game_state_base (cast `/Game/Assignment3/Blueprints/NewGameStateBase` (`GameplayStatics.GetGameState`))
    (:`then`
      (`/Game/Assignment3/Blueprints/NewGameStateBase.RPC_Multicast_ResetPlayers` _asnew_game_state_base)
      (set `self.NumButtonPressed` 0))
    (:`CastFailed`
      (`KismetSystemLibrary.PrintString` "cast failed"))))

(event `DestorySession`
  (bind _asnew_game_state_base (cast `/Game/Assignment3/Blueprints/NewGameStateBase` (`GameplayStatics.GetGameState`))
    (:`then`
      (`/Game/Assignment3/Blueprints/NewGameStateBase.RPC_Multicast_DestoryLeave` _asnew_game_state_base))
    (:`CastFailed`
      (`KismetSystemLibrary.PrintString` "cast failed"))))

(fn `ChoosePlayerStart`
  (params (Player :type "Controller Object Reference"))
  (returns (ReturnValue :type "Actor Object Reference"))
  (bind _outactors (`GameplayStatics.GetAllActorsOfClass` "/Script/Engine.PlayerStart"))
  (for _array_element _outactors
    (if (`KismetStringLibrary.EqualEqual_StrStr` (`KismetStringLibrary.Concat_StrStr` (`self.PlayerStartString`) (`KismetStringLibrary.Conv_IntToString` (`self.CurrentSpawnIndex`))) (`KismetStringLibrary.Conv_NameToString` (`PlayerStart.PlayerStartTag` _array_element)))
      (`/Engine/EditorBlueprintResources/StandardMacros.IncrementInt` (`self.CurrentSpawnIndex`)
        (:`  `
          (return _array_element))))))

(fn `OnRep_NumButtonPressed`)

(fn `UserConstructionScript`)