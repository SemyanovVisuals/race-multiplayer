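; BP_LaserAttach is a laser actor that projects a beam from its Body up to the first surface in front of it.
; On BeginPlay it applies LaserColor to the Laser particle effect.
; Every Tick it line traces on Visibility along Body's forward vector up to Range and sets the X of "Beam End" to the impact distance.
; The hit result is used without checking for a miss.
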(event `self.ReceiveBeginPlay`
  (`FXSystemComponent.SetColorParameter` (`self.Laser`) "Color" (`self.LaserColor`)))

(event `self.ReceiveTick`
  (params (DeltaSeconds :type "Float (single-precision)"))
  (bind _body (`self.Body`))
  (bind _returnvalue (`SceneComponent.K2_GetComponentLocation` _body))
  (bind _outhit (`KismetSystemLibrary.LineTraceSingle` _returnvalue (+ _returnvalue (* (`SceneComponent.GetForwardVector` _body) (`self.Range`))) "TraceTypeQuery1"))
  (`FXSystemComponent.SetVectorParameter` (`self.Laser`) "Beam End" (`KismetMathLibrary.MakeVector` (`KismetMathLibrary.Vector_Distance` (`SceneComponent.K2_GetComponentLocation` (`self.Body`)) (`.ImpactPoint` (`GameplayStatics.BreakHitResult` _outhit))))))

(fn `UserConstructionScript`)