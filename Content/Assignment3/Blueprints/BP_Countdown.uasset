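; BP_Countdown is a countdown actor that shows 3 down to 0 on a WB_Countdown widget, with beep sounds.
; StartCountdown plays the first beep and starts a looping timer on UpdateCountdown, which switches on SecondsElapsed to set the text and advance the counter.
; A different beep marks zero, then the next tick clears the timer and hides the widget component.
; ResetCountdown restores the text and counter, but not visibility.
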(event `self.ReceiveBeginPlay`)

(fn `ResetCountdown`
  (`self.UpdateWidgetText` "3")
  (set `self.SecondsElapsed` 0))

(fn `StartCountdown`
  (bind _returnvalue (`KismetSystemLibrary.K2_SetTimer` null "UpdateCountdown" 2.0 true))
  (set `self.Timer` _returnvalue)
  (`GameplayStatics.PlaySound2D` "/Game/Assignment3/Sounds/countdownbeep.countdownbeep" 1.0 1.0 0.0 null null))

(fn `UpdateCountdown`
  (locals (CurrentText :type Text :default "NSLOCTEXT(\"[1D22C430E37505D50CB40944BB289561]\", \"4BD2A20443DB8A659F6E1DB9FE23E493\", \"0\")"))
  (switch `int` (`self.SecondsElapsed`)
    (:`0`
      (`self.UpdateWidgetText` "2")
      (`self.UpdateTimerValues` :!label _label)
      (if (== (`self.SecondsElapsed`) 3)
        (`KismetSystemLibrary.PrintString` "Hello")
        (`GameplayStatics.PlaySound2D` "/Game/Assignment3/Sounds/finishcountdownbeep.finishcountdownbeep" 1.0 1.0 0.0 null null)
        (else
          (`GameplayStatics.PlaySound2D` "/Game/Assignment3/Sounds/countdownbeep.countdownbeep" 1.0 1.0 0.0 null null))))
    (:`1`
      (`self.UpdateWidgetText` "1")
      (goto _label))
    (:`2`
      (`self.UpdateWidgetText` "0")
      (goto _label))
    (:`3`
      (`self.UpdateTimerValues`))))

(fn `UpdateTimerValues`
  (bind _result (`/Engine/EditorBlueprintResources/StandardMacros.IncrementInt` (`self.SecondsElapsed`))
    (:`  `
      (bind _output_get (set `self.SecondsElapsed` _result))
      (if (>= _output_get 4)
        (`KismetSystemLibrary.K2_ClearAndInvalidateTimerHandle` (`self.Timer`))
        (`SceneComponent.SetVisibility` (`self.Widget`) false true)))))

(fn `UpdateWidgetText`
  (params (CurrentText :type Text))
  (bind _aswb_countdown (cast `/Game/Assignment3/UI/WB_Countdown` (`WidgetComponent.GetUserWidgetObject` (`self.Widget`))))
  (`TextBlock.SetText` (`/Game/Assignment3/UI/WB_Countdown.Countdown` _aswb_countdown) (`local.CurrentText`)))

(fn `UserConstructionScript`)