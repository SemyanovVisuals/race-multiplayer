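; Game state for a two-player VR match, with multicast-named events for countdown, finish, reset and leaving.
; Finish branches on authority and, guarded by DoOnce, spawns a small result menu at that side's player plus a large fixed one.
; Reset re-enables actions, returns the local pawn to its start, recenters the headset, clears menus and resets the countdown.
; Leaving opens the lobby level, with the host delaying briefly and calling DestroySession.
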(event `RPC_Multicast_StartCountdown`
  (bind _returnvalue (`GameplayStatics.GetActorOfClass` "/Game/Assignment3/Blueprints/BP_Countdown.BP_Countdown_C"))
  (bind _output_get (set `self.CounterDownWidget` _returnvalue))
  (`/Game/Assignment3/Blueprints/BP_Countdown.StartCountdown` _output_get))

(event `RPC_Multicast_FinishMessage`
  (params (Client0Won :type Boolean) (Client0Rotation :type "Rotator Structure") (Client1Rotation :type "Rotator Structure") (Client0Location :type "Vector Structure") (Client1Location :type "Vector Structure"))
  (`/Engine/EditorBlueprintResources/ActorMacros.Switch Has Authority`
    (:`Authority`
      (`/Engine/EditorBlueprintResources/StandardMacros.DoOnce` false :!label _label
        (:`Completed`
          (`|ExecutionSequence`
            (:`then_0`
              (bind _returnvalue (`|SpawnActorFromClass` "/Game/Assignment3/Blueprints/BP_FinishMenu.BP_FinishMenu_C" (`KismetMathLibrary.MakeTransform` Client0Location Client0Rotation (0.25 0.25 0.25)) "Undefined" "MultiplyWithRoot" null null))
              (bind _aswb_finish (cast `/Game/Assignment3/UI/WB_Finish` (`WidgetComponent.GetUserWidgetObject` (`self.GetComponentByClass` _returnvalue "/Script/UMG.WidgetComponent")))
                (:`then`
                  (`/Game/Assignment3/UI/WB_Finish.UpdateFinishMessageUI` _aswb_finish Client0Won))
                (:`CastFailed`
                  (`KismetSystemLibrary.PrintString` "cast failed"))))
            (:`then_1`
              (bind _returnvalue_2 (`|SpawnActorFromClass` "/Game/Assignment3/Blueprints/BP_FinishMenu.BP_FinishMenu_C" (`KismetMathLibrary.MakeTransform` (3467.0 -166.0 800.0) (struct :`Yaw` 180.0) (2.0 2.0 2.0)) "Undefined" "MultiplyWithRoot" null null))
              (bind _aswb_finish_2 (cast `/Game/Assignment3/UI/WB_Finish` (`WidgetComponent.GetUserWidgetObject` (`self.GetComponentByClass` _returnvalue_2 "/Script/UMG.WidgetComponent")))
                (:`then`
                  (`/Game/Assignment3/UI/WB_Finish.UpdateFinishMessageUI` _aswb_finish_2 Client0Won))
                (:`CastFailed`
                  (`KismetSystemLibrary.PrintString` "cast failed"))))))))
    (:`Remote`
      (`/Engine/EditorBlueprintResources/StandardMacros.DoOnce` false :!label _label_2
        (:`Completed`
          (`|ExecutionSequence`
            (:`then_0`
              (bind _returnvalue_3 (`|SpawnActorFromClass` "/Game/Assignment3/Blueprints/BP_FinishMenu.BP_FinishMenu_C" (`KismetMathLibrary.MakeTransform` Client1Location Client1Rotation (0.25 0.25 0.25)) "Undefined" "MultiplyWithRoot" null null))
              (bind _aswb_finish_3 (cast `/Game/Assignment3/UI/WB_Finish` (`WidgetComponent.GetUserWidgetObject` (`self.GetComponentByClass` _returnvalue_3 "/Script/UMG.WidgetComponent")))
                (:`then`
                  (`/Game/Assignment3/UI/WB_Finish.UpdateFinishMessageUI` _aswb_finish_3 Client0Won))
                (:`CastFailed`
                  (`KismetSystemLibrary.PrintString` "cast failed"))))
            (:`then_1`
              (bind _returnvalue_4 (`|SpawnActorFromClass` "/Game/Assignment3/Blueprints/BP_FinishMenu.BP_FinishMenu_C" (`KismetMathLibrary.MakeTransform` (3467.0 -1616.0 800.0) (struct :`Yaw` 180.0) (2.0 2.0 2.0)) "Undefined" "MultiplyWithRoot" null null))
              (bind _aswb_finish_4 (cast `/Game/Assignment3/UI/WB_Finish` (`WidgetComponent.GetUserWidgetObject` (`self.GetComponentByClass` _returnvalue_4 "/Script/UMG.WidgetComponent")))
                (:`then`
                  (`/Game/Assignment3/UI/WB_Finish.UpdateFinishMessageUI` _aswb_finish_4 Client0Won))
                (:`CastFailed`
                  (`KismetSystemLibrary.PrintString` "cast failed"))))))))))

(event `RPC_Multicast_ResetPlayers`
  (bind _asbp_vrpawn (cast `/Game/Assignment3/Blueprints/BP_VRPawn` (`GameplayStatics.GetPlayerPawn` 0))
    (:`then`
      (bind _menureference (`/Game/Assignment3/Blueprints/BP_VRPawn.MenuReference` _asbp_vrpawn))
      (if (`KismetSystemLibrary.IsValid` _menureference)
        (bind _aswb_widget_menu (cast `/Game/Assignment3/UI/WB_WidgetMenu` (`WidgetComponent.GetUserWidgetObject` (`/Game/VRTemplate/Blueprints/Menu.Widget` _menureference)))
          (:`then`
            _)
          (:`CastFailed`
            (`KismetSystemLibrary.PrintString` "Cast failed Text")))
        (set `Widget.bIsEnabled` true (`/Game/Assignment3/UI/WB_WidgetMenu.ReadyToPlayButton` _aswb_widget_menu))
        (bind _asbp_vrpawn_2 (cast `/Game/Assignment3/Blueprints/BP_VRPawn` (`GameplayStatics.GetPlayerPawn` 0))
          (:`then`
            (set `/Game/Assignment3/Blueprints/BP_VRPawn.bIsActionAvailable` true _asbp_vrpawn_2 :!label _label_3)
            (bind _asbp_vrpawn_3 (cast `/Game/Assignment3/Blueprints/BP_VRPawn` (`GameplayStatics.GetPlayerPawn` 0))
              (:`then`
                (bind _startlocationactorstorage (`/Game/Assignment3/Blueprints/BP_VRPawn.StartLocationActorStorage` _asbp_vrpawn_3))
                (`KismetSystemLibrary.PrintString` (`KismetStringLibrary.Conv_VectorToString` _startlocationactorstorage))
                (`self.K2_SetActorLocation` _asbp_vrpawn_3 _startlocationactorstorage false false)
                (`HeadMountedDisplayFunctionLibrary.ResetOrientationAndPosition` 0.0)
                (bind _returnvalue (`GameplayStatics.GetActorOfClass` "/Game/Assignment3/Blueprints/BP_Countdown.BP_Countdown_C"))
                (set `self.CounterDownWidget` _returnvalue)
                (bind _outactors (`GameplayStatics.GetAllActorsOfClass` "/Game/Assignment3/Blueprints/BP_FinishMenu.BP_FinishMenu_C"))
                (for _array_element _outactors
                  (`self.K2_DestroyActor` _array_element)
                  (`|ExecutionSequence`
                    (:`then_0`
                      (goto _label_2 :!via `Reset`))
                    (:`then_1`
                      (goto _label :!via `Reset`))
                    (:`then_2`
                      (bind _returnvalue_2 (`GameplayStatics.GetActorOfClass` "/Game/Assignment3/Blueprints/BP_Countdown.BP_Countdown_C"))
                      (`SceneComponent.SetVisibility` (`/Game/Assignment3/Blueprints/BP_Countdown.Widget` _returnvalue_2) true true)
                      (`/Game/Assignment3/Blueprints/BP_Countdown.ResetCountdown` _returnvalue_2)))))
              (:`CastFailed`
                (`KismetSystemLibrary.PrintString` " cast failed"))))
          (:`CastFailed`
            (`KismetSystemLibrary.PrintString` "cast failed")))
        (else
          (goto _label_3))))
    (:`CastFailed`
      (`KismetSystemLibrary.PrintString` "cast failed"))))

(event `RPC_Multicast_DestoryLeave`
  (`/Engine/EditorBlueprintResources/ActorMacros.Switch Has Authority`
    (:`Authority`
      (`KismetSystemLibrary.Delay` 0.5))
    (:`Remote`
      _))
  (`GameplayStatics.OpenLevel` "LVL_GameLobby2")
  (`/Engine/EditorBlueprintResources/ActorMacros.Switch Has Authority`
    (:`Authority`
      (`DestroySessionCallbackProxy.DestroySession` (`GameplayStatics.GetPlayerController` 0)))))

(fn `OnRep_DEBUG_Countdown`)

(fn `UserConstructionScript`)